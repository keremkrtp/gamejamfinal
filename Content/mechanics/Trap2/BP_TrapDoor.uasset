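; BP_TrapDoor is a crushing gate trap that raises and lowers its mesh vertically.
; OpenGate plays the DoorAnim timeline to lift the StaticMesh, while SmashGate reverses it and sets IsClosing.
; When the player character begins overlapping CrushZone with IsClosing set, the level restarts through a console command, followed by a 2D sound call.
; IsClosing clears only on OpenGate, so the zone stays lethal after the gate finishes closing.
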(event OnComponentBeginOverlap(CrushZone)
  (params (OverlappedComponent :type Primitive%20Component%20Object%20Reference) (OtherActor :type Actor%20Object%20Reference) (OtherComp :type Primitive%20Component%20Object%20Reference) (OtherBodyIndex :type Integer) (bFromSweep :type Boolean) (SweepResult :type Hit%20Result%20Structure%20%28by%20ref%29))
  (Utilities|Casting|CastToBP_ThirdPersonCharacter OtherActor)
  (if (Variables|Default|GetIsClosing)
    (Development|ExecuteConsoleCommand "RestartLevel" 0)
    (Audio|PlaySound2D 0 1.0 1.0 0.0 0 0)))

(event Custom|OpenGate
  (Variables|Default|SetIsClosing false)
  (bind _newtrack_0 (Timeline|DoorAnim Play)
    (:Update
      (Transformation|SetRelativeLocation (Variables|Default|GetStaticMesh) (Math|Vector|Lerp(Vector) "0, 0, 0" "0.000000,0.000000,300.000000" _newtrack_0) false false))))

(event Custom|SmashGate
  (Variables|Default|SetIsClosing true)
  (bind _newtrack_0 (Timeline|DoorAnim Reverse)
    (:Update
      (Transformation|SetRelativeLocation (Variables|Default|GetStaticMesh) (Math|Vector|Lerp(Vector) "0, 0, 0" "0.000000,0.000000,300.000000" _newtrack_0) false false))))

(event EventBeginPlay)

(event Collision|EventActorBeginOverlap
  (params (OtherActor :type Actor%20Object%20Reference)))

(event EventTick
  (params (DeltaSeconds :type Float%20%28single-precision%29)))

(fn ConstructionScript)