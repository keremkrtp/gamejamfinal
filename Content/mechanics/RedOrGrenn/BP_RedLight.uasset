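; BP_RedLight is a Red Light, Green Light hazard that restarts the level when the player moves during red.
; A self-repeating ToggleLight event swaps the mesh material and IsRedLight flag, with a random-length green phase and fixed-length red phase.
; DetectionZone overlaps track whether the third-person character is in range.
; While in range during red, Tick waits a short grace Delay, then checks player velocity and runs the RestartLevel console command.
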(event OnComponentBeginOverlap(DetectionZone)
  (params (OverlappedComponent :type Primitive%20Component%20Object%20Reference) (OtherActor :type Actor%20Object%20Reference) (OtherComp :type Primitive%20Component%20Object%20Reference) (OtherBodyIndex :type Integer) (bFromSweep :type Boolean) (SweepResult :type Hit%20Result%20Structure%20%28by%20ref%29))
  (Utilities|Casting|CastToBP_ThirdPersonCharacter OtherActor)
  (Variables|Default|SetIsPlayerInRange true))

(event OnComponentEndOverlap(DetectionZone)
  (params (OverlappedComponent :type Primitive%20Component%20Object%20Reference) (OtherActor :type Actor%20Object%20Reference) (OtherComp :type Primitive%20Component%20Object%20Reference) (OtherBodyIndex :type Integer))
  (Utilities|Casting|CastToBP_ThirdPersonCharacter OtherActor)
  (Variables|Default|SetIsPlayerInRange false))

(event Custom|ToggleLight
  (Rendering|Material|SetMaterial (Variables|Default|GetStaticMesh) 0 "/Game/ThirdPerson/MI_ThirdPersonColWay.MI_ThirdPersonColWay")
  (Variables|Default|SetIsRedLight false)
  (Variables|Default|SetPointLight 0)
  (Utilities|FlowControl|Delay (Math|Random|RandomFloatinRange 2.0 5.0))
  (Rendering|Material|SetMaterial (Variables|Default|GetStaticMesh) 0 "/Game/StarterContent/Props/Materials/M_Lamp.M_Lamp")
  (Variables|Default|SetIsRedLight true)
  (Utilities|FlowControl|Delay 3.0)
  (CallFunction|ToggleLight))

(event EventBeginPlay
  (CallFunction|ToggleLight))

(event EventTick
  (params (DeltaSeconds :type Float%20%28single-precision%29))
  (if (Variables|Default|GetIsPlayerInRange)
    (if (Variables|Default|GetIsRedLight)
      (Utilities|FlowControl|Delay 0.4)
      (if (> (Math|Vector|VectorLength (Transformation|GetVelocity (Game|GetPlayerCharacter 0))) 1e+01)
        (Development|ExecuteConsoleCommand "RestartLevel" 0)))))

(fn ConstructionScript)