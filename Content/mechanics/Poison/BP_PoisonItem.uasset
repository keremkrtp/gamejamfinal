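; BP_PoisonItem is a poison pickup that disorients the player on contact.
; Overlap with its sphere sets BP_ThirdPersonCharacter's ControlMultiplier to -1, starts a drunk camera shake and prints a Turkish dizziness message.
; The item hides its mesh and disables collision, then after a delay sets the multiplier to 10 (not 1) and destroys itself.
; The camera shake is never explicitly stopped here.
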(event OnComponentBeginOverlap(Sphere)
  (params (OverlappedComponent :type Primitive%20Component%20Object%20Reference) (OtherActor :type Actor%20Object%20Reference) (OtherComp :type Primitive%20Component%20Object%20Reference) (OtherBodyIndex :type Integer) (bFromSweep :type Boolean) (SweepResult :type Hit%20Result%20Structure%20%28by%20ref%29))
  (bind _asbp_third_person_character (Utilities|Casting|CastToBP_ThirdPersonCharacter OtherActor))
  (Variables|/Game/ThirdPerson/Blueprints/BP_ThirdPersonCharacter.BP_ThirdPersonCharacter_C|SetControlMultiplier _asbp_third_person_character -1.0)
  (CameraShakes|StartCameraShake (Game|GetPlayerCameraManager 0) "/Game/mechanics/Poison/BP_DrunkShake.BP_DrunkShake_C" 1.0 "CameraLocal" "0, 0, 0")
  (Development|SetHiddeninGame (Variables|Default|GetStaticMesh) true false)
  (Collision|SetCollisionEnabled (Variables|Default|GetSphere) "NoCollision")
  (Collision|SetCollisionEnabled (Variables|Default|GetStaticMesh) "NoCollision")
  (Development|PrintString "AHHH!! BAŞIM DÖNÜYOR")
  (Utilities|FlowControl|Delay 1e+01)
  (Variables|/Game/ThirdPerson/Blueprints/BP_ThirdPersonCharacter.BP_ThirdPersonCharacter_C|SetControlMultiplier _asbp_third_person_character 1e+01)
  (Actor|DestroyActor))

(event EventBeginPlay)

(event Collision|EventActorBeginOverlap
  (params (OtherActor :type Actor%20Object%20Reference)))

(event EventTick
  (params (DeltaSeconds :type Float%20%28single-precision%29)))

(fn ConstructionScript)