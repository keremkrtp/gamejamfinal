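; BP_CrushingWalls1 is a crushing-walls trap that restarts the level when it catches the player character.
; The ActivateTrap event plays a timeline that lerps the left and right walls toward each other along local X.
; When the timeline finishes, actors overlapping the Box are checked, and a BP_ThirdPersonCharacter among them triggers the RestartLevel console command.
; The file contains no reset or reverse motion for the walls.
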(event Custom|ActivateTrap
  (bind _newtrack_0 (Timeline|Timeline Play)
    (:Update
      (Transformation|SetRelativeLocation (Variables|Default|GetLeftWall) (Math|Vector|MakeVector (Math|Float|Lerp 1.9e+02 0.0 _newtrack_0) 0.0 0.0) false false)
      (Transformation|SetRelativeLocation (Variables|Default|GetRightWall) (Math|Vector|MakeVector (Math|Float|Lerp -2e+02 -3e+01 _newtrack_0) 0.0 0.0) false false))
    (:Finished
      (for _array_element (Collision|GetOverlappingActors (Variables|Default|GetBox) 0 :!class /Script/Engine.PrimitiveComponent)
        (Utilities|Casting|CastToBP_ThirdPersonCharacter _array_element)
        (Development|ExecuteConsoleCommand "RestartLevel" 0)))))

(event EventBeginPlay)

(event Collision|EventActorBeginOverlap
  (params (OtherActor :type Actor%20Object%20Reference)))

(event EventTick
  (params (DeltaSeconds :type Float%20%28single-precision%29)))

(fn ConstructionScript)